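; MainCharacter is a player character Blueprint that provides basic movement and camera look through axis inputs.
; Forward/Backward and Right/Left feed AddMovementInput using vectors built from the control rotation's yaw alone, so movement follows the camera heading without being affected by pitch.
; Turn and LookUp pass their axis values directly to controller yaw and pitch input.
; The construction script is empty.
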(event `InputAxis|Forward/Backward`
  (params (AxisValue :type "Float (single-precision)"))
  ;[1 1 1] Basic Movement
  (`self.AddMovementInput` (`KismetMathLibrary.GetForwardVector` (`KismetMathLibrary.MakeRotator` 0.0 0.0 (.yaw (`self.GetControlRotation`)))) AxisValue))

(event `InputAxis|Right/Left`
  (params (AxisValue :type "Float (single-precision)"))
  ;[1 1 1] Basic Movement
  (`self.AddMovementInput` (`KismetMathLibrary.GetRightVector` (`KismetMathLibrary.MakeRotator` 0.0 0.0 (.yaw (`self.GetControlRotation`)))) AxisValue))

(event `InputAxis|Turn`
  (params (AxisValue :type "Float (single-precision)"))
  ;[1 1 1] Basic Camera Movement
  (`self.AddControllerYawInput` AxisValue))

(event `InputAxis|LookUp`
  (params (AxisValue :type "Float (single-precision)"))
  ;[1 1 1] Basic Camera Movement
  (`self.AddControllerPitchInput` AxisValue))

(fn `UserConstructionScript`)